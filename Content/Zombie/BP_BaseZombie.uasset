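; Base zombie enemy with move-to-player, melee attack and death events, tied to AI through the "seeingTarget?" blackboard flag.
; TargetMoveto sets the flag when the move succeeds; BeginPlay and attack completion clear it.
; Attack stops movement and plays a montage, whose notify sphere-traces for pawns to apply damage.
; OnDie plays a death montage before destroying the actor, but AnyDamage is empty and the DT_Zombie health logic is disconnected.
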(event Custom|OnDie
  ;[1 1 1] 사망
  (Pawn|Components|CharacterMovement|DisableMovement (Variables|Character|GetCharacterMovement))
  (Collision|SetActorEnableCollision false)
  (Animation|Montage|PlayMontage (Variables|Character|GetMesh) "/Game/zombbb/Zombie_Dying_Montage.Zombie_Dying_Montage"
    (:then
      (Utilities|FlowControl|Delay 3.0)
      (Actor|DestroyActor))))

(event EventBeginPlay
  (AI|Components|Blackboard|SetValueasBool (AI|GetBlackboard 0) (Utilities|Name|MakeLiteralName "seeingTarget?") false))

(event EventTargetMoveto
  (AI|AIMoveTo self "0, 0, 0" (Game|GetPlayerController 0) 1e+01 false
    (:OnSuccess
      (Development|PrintString "성공")
      (AI|Components|Blackboard|SetValueasBool (AI|GetBlackboard 0) (Utilities|Name|MakeLiteralName "seeingTarget?") true))))

(event EventAttack
  (bind _mesh (Variables|Character|GetMesh))
  (bind _returnvalue (Transformation|GetWorldRotation _mesh))
  (bind _returnvalue_2 (Transformation|GetWorldLocation _mesh))
  (bind _returnvalue_3 (Math|Vector|GetForwardVector _returnvalue))
  (bind _returnvalue_4 (Math|Conversions|RotationFromXVector _returnvalue_3))
  (bind (_roll _pitch _yaw) (Math|Rotator|BreakRotator _returnvalue_4))
  ;[1 1 1] 공격
  (Components|Movement|StopMovementImmediately (Variables|Character|GetCharacterMovement))
  (if (not (Variables|Default|GetisAttack?))
    (Animation|Montage|PlayMontage (Variables|Character|GetMesh) "/Game/zombbb/ANM_Attack.ANM_Attack"
      (:then
        (Variables|Default|SetisAttack? true))
      (:OnCompleted
        (Variables|Default|SetisAttack? false)
        (AI|Components|Blackboard|SetValueasBool (AI|GetBlackboard 0) (Utilities|Name|MakeLiteralName "seeingTarget?") false))
      (:OnNotifyBegin
        (bind (_outhit _returnvalue_5) (Collision|SphereTraceForObjects _returnvalue_2 (+ _returnvalue_2 (* (Math|Rotator|MakeRotator _roll _pitch (+ _yaw 9e+01)) 1.5e+02)) 45.0 (Utilities|Array|MakeArray "ObjectTypeQuery3") false 0 "ForDuration" true "(R=1.000000,G=0.000000,B=0.000000,A=1.000000)" "(R=0.000000,G=1.000000,B=0.000000,A=1.000000)" 2.0))
        (if _returnvalue_5
          (Game|Damage|ApplyDamage (.HitActor (Collision|BreakHitResult _outhit)) 1e+01 0 0))))))

(event Game|Damage|EventAnyDamage
  (params (Damage :type Float%20%28single-precision%29) (DamageType :type Damage%20Type%20Object%20Reference) (InstigatedBy :type Controller%20Object%20Reference) (DamageCauser :type Actor%20Object%20Reference))
  ;[1 1 1] 체력 맞았을때
)

(fn ConstructionScript)