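; Base dash-attacking zombie character that exchanges attack state with its AI through Blackboard keys, with delayed Wait and Idle events.
; Attack plays a run montage while a looping timer fires five forward launches, then clears CanAttack.
; Montage notifies trigger a sphere trace that damages the pawn hit.
; OnDie plays a death montage and destroys the actor, but damage and health logic is unwired, and the movement-tuning functions are uncalled here.
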(event Custom|OnDie
  ;[1 1 1] 사망
  (Pawn|Components|CharacterMovement|DisableMovement (Variables|Character|GetCharacterMovement))
  (Collision|SetActorEnableCollision false)
  (Animation|Montage|PlayMontage (Variables|Character|GetMesh) "/Game/zombbb/Zombie_Dying_Montage.Zombie_Dying_Montage"
    (:then
      (Utilities|FlowControl|Delay 3.0)
      (Actor|DestroyActor))))

(event Custom|AddForce
  (if (>= (Variables|Default|GetDashCount) 1)
    (CallFunction|Dash)
    (Variables|Default|SetDashCount (- (Variables|Default|GetDashCount) 1))
    (Development|PrintString (Utilities|String|ToString(Integer) (Variables|Default|GetDashCount)))
    (else
      (Utilities|Time|ClearandInvalidateTimerbyHandle (stale EventAttack _returnvalue))
      (AI|Components|Blackboard|SetValueasBool (AI|GetBlackboard 0) (Utilities|Name|MakeLiteralName "CanAttack") false))))

(event EventBeginPlay
  (bind _returnvalue (Utilities|GetDataTableRow "/Game/Data/Zombie/DT_Zombie.DT_Zombie" "BaseZombie")))

(event EventWait
  (Utilities|FlowControl|Delay 0.5)
  (AI|Components|Blackboard|SetValueasBool (AI|GetBlackboard 0) (Utilities|Name|MakeLiteralName "Wait") false))

(event EventAttack
  ;[1 1 1] 공격
  (if (not (Variables|Default|GetisAttack?))
    (Components|Movement|StopMovementImmediately (Variables|Character|GetCharacterMovement))
    (Animation|Montage|PlayMontage (Variables|Character|GetMesh) "/Game/Zombie/Dash/Standard_Run1_Montage.Standard_Run1_Montage"
      (:then
        (Variables|Default|SetisAttack? true)
        (Variables|Default|SetDashCount 5)
        (bind _returnvalue (Utilities|Time|SetTimerbyEvent (delegate Custom|AddForce) 0.1 true)))
      (:OnCompleted
        (Variables|Default|SetisAttack? false)
        (AI|Components|Blackboard|SetValueasBool (AI|GetBlackboard 0) (Utilities|Name|MakeLiteralName "seeingTarget?") false))
      (:OnNotifyBegin
        (CallFunction|DashAttack)))))

(event EventIdle
  (Utilities|FlowControl|Delay 5.0)
  (AI|Components|Blackboard|SetValueasBool (AI|GetBlackboard 0) (Utilities|Name|MakeLiteralName "CanAttack") true)
  (AI|Components|Blackboard|SetValueasBool (AI|GetBlackboard 0) (Utilities|Name|MakeLiteralName "Wait") true))

(event Game|Damage|EventAnyDamage
  (params (Damage :type Float%20%28single-precision%29) (DamageType :type Damage%20Type%20Object%20Reference) (InstigatedBy :type Controller%20Object%20Reference) (DamageCauser :type Actor%20Object%20Reference))
  ;[1 1 1] 체력 맞았을때
)

(fn ConstructionScript)

(fn SetMovement
  (bind _charactermovement (Variables|Character|GetCharacterMovement))
  (Variables|/Script/Engine.CharacterMovementComponent|SetMaxWalkSpeed _charactermovement 5e+03)
  (Variables|/Script/Engine.CharacterMovementComponent|SetMaxAcceleration _charactermovement 4096.0)
  (Variables|/Script/Engine.CharacterMovementComponent|SetBrakingFrictionFactor _charactermovement 0.2)
  (Variables|/Script/Engine.CharacterMovementComponent|SetBrakingDecelerationWalking _charactermovement 512.0))

(fn RetrunMovement
  (bind _charactermovement (Variables|Character|GetCharacterMovement))
  (Variables|/Script/Engine.CharacterMovementComponent|SetMaxWalkSpeed _charactermovement 6e+02)
  (Variables|/Script/Engine.CharacterMovementComponent|SetMaxAcceleration _charactermovement 2048.0)
  (Variables|/Script/Engine.CharacterMovementComponent|SetBrakingFrictionFactor _charactermovement 2.0)
  (Variables|/Script/Engine.CharacterMovementComponent|SetBrakingDecelerationWalking _charactermovement 2048.0))

(fn Dash
  (Character|LaunchCharacter (* (Transformation|GetActorForwardVector) (Variables|Default|GetDeshStren)) true false))

(fn DashAttack
  (bind _mesh (Variables|Character|GetMesh))
  (bind _returnvalue (Transformation|GetWorldRotation _mesh))
  (bind _returnvalue_2 (Transformation|GetWorldLocation _mesh))
  (bind _returnvalue_3 (Math|Vector|GetForwardVector _returnvalue))
  (bind _returnvalue_4 (Math|Conversions|RotationFromXVector _returnvalue_3))
  (bind (_roll _pitch _yaw) (Math|Rotator|BreakRotator _returnvalue_4))
  (bind (_outhit _returnvalue_5) (Collision|SphereTraceForObjects _returnvalue_2 (+ _returnvalue_2 (* (Math|Rotator|MakeRotator _roll _pitch (+ _yaw 9e+01)) 7.5e+02)) 45.0 (Utilities|Array|MakeArray "ObjectTypeQuery3") false 0 "ForDuration" true "(R=1.000000,G=0.000000,B=0.000000,A=1.000000)" "(R=0.000000,G=1.000000,B=0.000000,A=1.000000)" 2.0))
  (if _returnvalue_5
    (Game|Damage|ApplyDamage (.HitActor (Collision|BreakHitResult _outhit)) 1e+01 0 0)))