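; BP_ZombieCreeper is an exploding zombie that swells, then deals damage around itself and dies.
; Attack, skipped if IsAttack is true, sets that blackboard key and starts a timeline that scales up its Sphere.
; After a short delay, a zero-length sphere trace damages only the first Pawn hit.
; It dies either way, disabling movement and collision, playing a dying montage, then destroying itself.
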(event Custom|OnDie
  (Pawn|Components|CharacterMovement|DisableMovement (Variables|Character|GetCharacterMovement))
  (Collision|SetActorEnableCollision false)
  (Animation|Montage|PlayMontage (Variables|Character|GetMesh) "/Game/zombbb/Zombie_Dying_Montage.Zombie_Dying_Montage"
    (:then
      (Utilities|FlowControl|Delay 3.0)
      (Actor|DestroyActor))))

(event Custom|OnExplode
  (bind _alpha (Timeline|TL_Grow Play)
    (:Update
      (Transformation|SetWorldScale3D (Variables|Default|GetSphere) (+ (* (Variables|Default|GetAddScale) _alpha) (Variables|Default|GetFScale))))))

(event EventAttack
  (if (not (Variables|Default|GetisAttack?))
    (AI|Components|Blackboard|SetValueasBool (AI|GetBlackboard 0) (Utilities|Name|MakeLiteralName "IsAttack") true)
    (CallFunction|OnExplode)
    (Utilities|FlowControl|Delay 2.0)
    (bind (_outhit _returnvalue) (Collision|SphereTraceForObjects (Transformation|GetActorLocation) (* (Transformation|GetActorLocation) "1.000000,1.000000,1.000000") 3e+02 (Utilities|Array|MakeArray "ObjectTypeQuery3") false 0 "ForDuration" true "(R=1.000000,G=0.000000,B=0.000000,A=1.000000)" "(R=0.000000,G=1.000000,B=0.000000,A=1.000000)" 2.0))
    (if _returnvalue
      (Game|Damage|ApplyDamage (.HitActor (Collision|BreakHitResult _outhit)) 1e+02 0 0)
      (CallFunction|OnDie)
      (else
        (CallFunction|OnDie)))))

(fn ConstructionScript)