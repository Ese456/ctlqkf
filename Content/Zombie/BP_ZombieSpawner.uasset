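; Zombie spawner actor that periodically spawns waves of four zombie types (Base, Run, Creeper, Desh) at its own location.
; A looping timer triggers spawns, with per-type counts read from DT_WaveZombie rows for the current wave.
; With AutoStartLoop, it starts the loop and binds to a TimerActor, whose updates advance the wave at TypeInterval multiples.
; Spawning only runs when UseTargetPoint is off.
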(event Custom|SpawnNow
  ;[1 1 1] 몹 스폰 세팅
  (if (not (Variables|Default|GetUseTargetPoint))
    (CallFunction|SpawnZombie "NewEnumerator0")
    (CallFunction|SpawnZombie "NewEnumerator2")
    (CallFunction|SpawnZombie "NewEnumerator1")
    (CallFunction|SpawnZombie "NewEnumerator3")))

(event Custom|OnTimerTicked
  (params (CurrentTime :type Float%20%28single-precision%29))
  (if (<= (Math|Integer|%(Integer) (Math|Float|Truncate CurrentTime) (Math|Float|Truncate (Variables|Default|GetTypeInterval))) 0)
    (Variables|Default|SetZombieSpawnWave (+ (Variables|Default|GetZombieSpawnWave) 1))))

(event Custom|StartSpawnLoop
  ;[1 1 1] SpawnTick 마다 몹스폰
  (Utilities|Time|ClearandInvalidateTimerbyHandle (Variables|Default|GetSpawnTimerHandle))
  (bind _returnvalue (Utilities|Time|SetTimerbyFunctionName 0 "SpawnMob" (Variables|Default|GetSpawnTick) true))
  (Variables|Default|SetSpawnTimerHandle _returnvalue))

(event Custom|OnSpawnTimer
  ;[1 1 1] Comment
  (CallFunction|SpawnNow))

(event Custom|StopSpawnLoop
  ;[1 1 1] Comment
  (Utilities|Time|ClearandInvalidateTimerbyHandle (Variables|Default|GetSpawnTimerHandle)))

(event Custom|RestartSpawnLoop
  ;[1 1 1] Comment
  (CallFunction|StopSpawnLoop)
  (CallFunction|StartSpawnLoop))

(event EventBeginPlay
  ;[1 1 1] Comment
  (CallFunction|SetZombie)
  (if (Variables|Default|GetAutoStartLoop)
    (CallFunction|StartSpawnLoop)
    (bind _outactors (Actor|GetAllActorsOfClass "/Script/ctlqkf.TimerActor"))
    (EventDispatchers|BindEventtoOnTimerUpdated (Utilities|Array|Get(acopy) _outactors) (delegate Custom|OnTimerTicked))))

(fn ConstructionScript)

(fn GetRandomPointinNavVolume)

(fn SpawnMob
  (CallFunction|SpawnNow))

(fn SetZombie
  (bind _returnvalue (Utilities|GetDataTableRow "/Game/Data/Zombie/DT_WaveZombie.DT_WaveZombie" "BaseZomibe")
    (:then
      (Variables|DataTable|SetRowBaseZombie _returnvalue)
      (bind _returnvalue_2 (Utilities|GetDataTableRow "/Game/Data/Zombie/DT_WaveZombie.DT_WaveZombie" "RunZombie")
        (:then
          (Variables|DataTable|SetRowRunZombie _returnvalue_2)
          (bind _returnvalue_3 (Utilities|GetDataTableRow "/Game/Data/Zombie/DT_WaveZombie.DT_WaveZombie" "Creeper")
            (:then
              (Variables|DataTable|SetRowCreeper _returnvalue_3)
              (bind _returnvalue_4 (Utilities|GetDataTableRow "/Game/Data/Zombie/DT_WaveZombie.DT_WaveZombie" "Desh")
                (:then
                  (Variables|DataTable|SetRowDesh _returnvalue_4))))))))))

(fn SetZombiePos
  (return (Math|Transform|MakeTransform (Transformation|GetWorldLocation (Variables|Default|GetDefaultSceneRoot)) (Math|Conversions|RotationFromXVector (Variables|Default|GetSpawnRotation)))))

(fn GetPower
  (params (Type :type E_Zomibe%20Enum :default "NewEnumerator0"))
  (switch Utilities|FlowControl|Switch|SwitchonE_Zomibe Type
    (:NewEnumerator0
      (Variables|DataTable|SetCurrentZombie (Variables|DataTable|GetRowBaseZombie)))
    (:NewEnumerator2
      (Variables|DataTable|SetCurrentZombie (Variables|DataTable|GetRowRunZombie)))
    (:NewEnumerator1
      (Variables|DataTable|SetCurrentZombie (Variables|DataTable|GetRowCreeper)))
    (:NewEnumerator3
      (Variables|DataTable|SetCurrentZombie (Variables|DataTable|GetRowDesh))))
  (switch int (Variables|Default|GetZombieSpawnWave)
    (:0
      (Variables|Default|SetCurrentPower (.Time0 (Utilities|Struct|BreakS_Wave (Variables|DataTable|GetCurrentZombie)))))
    (:1
      (Variables|Default|SetCurrentPower (.Time2 (Utilities|Struct|BreakS_Wave (Variables|DataTable|GetCurrentZombie)))))
    (:2
      (Variables|Default|SetCurrentPower (.Time4 (Utilities|Struct|BreakS_Wave (Variables|DataTable|GetCurrentZombie)))))
    (:3
      (Variables|Default|SetCurrentPower (.Time6 (Utilities|Struct|BreakS_Wave (Variables|DataTable|GetCurrentZombie)))))
    (:4
      (Variables|Default|SetCurrentPower (.Time8 (Utilities|Struct|BreakS_Wave (Variables|DataTable|GetCurrentZombie)))))
    (:5
      (Variables|Default|SetCurrentPower (.Time10 (Utilities|Struct|BreakS_Wave (Variables|DataTable|GetCurrentZombie))))))
  (return (Variables|Default|GetCurrentPower)))

(fn SpawnZombie
  (params (NewParam :type E_Zomibe%20Enum :default "NewEnumerator0"))
  (bind _currentpower (CallFunction|GetPower NewParam))
  (Variables|Default|SetCurrentPower _currentpower)
  (if (> (Variables|Default|GetCurrentPower) 0)
    (switch Utilities|FlowControl|Switch|SwitchonE_Zomibe NewParam
      (:NewEnumerator0
        (Variables|Default|SetCurrenntZombieClass "/Game/Zombie/BP_BaseZombie.BP_BaseZombie_C"))
      (:NewEnumerator2
        (Variables|Default|SetCurrenntZombieClass "/Game/Zombie/BP_ZombieRun.BP_ZombieRun_C"))
      (:NewEnumerator1
        (Variables|Default|SetCurrenntZombieClass "/Game/Zombie/BP_ZombieCreeper.BP_ZombieCreeper_C"))
      (:NewEnumerator3
        (Variables|Default|SetCurrenntZombieClass "/Game/Zombie/BP_BaseDesh.BP_BaseDesh_C")))
    (bind _zombiepos (CallFunction|SetZombiePos))
    (for _index (range 1 (Variables|Default|GetCurrentPower))
      (Game|SpawnActorfromClass (Variables|Default|GetCurrenntZombieClass) _zombiepos "AlwaysSpawn" "MultiplyWithRoot" 0 0))))